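; Actor Blueprint that avateers a poseable mesh from Kinect body tracking.
; On BeginPlay it copies its Smoothing setting to the KinectPoseableMesh and configures rotation-spike smoothing parameters on the Kinect interface.
; Each Tick it fetches the centered body and, while that body is tracked, assigns it as the mesh's target body.
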(event `self.ReceiveBeginPlay`
  ;[1 1 1] Configure Kinect Poseable Mesh smoothing field
  (set `KinectPoseableMeshComponent.IsSmoothing` (`self.Smoothing`) (`self.KinectPoseableMesh`))
  (`KinectInterfaceComponent.SetSmoothingParameters` (`self.KinectInterface`) 0.0 0.5))

(event `self.ReceiveTick`
  (params (DeltaSeconds :type "Float (single-precision)"))
  ;[1 1 1] Update the Kinect Poseable Mesh to pull data from current centered body
  (bind (_centeredbody _istracked) (`KinectInterfaceComponent.GetCenteredBody` (`self.KinectInterface`)))
  (if _istracked
    (set `KinectPoseableMeshComponent.TargetBody` _centeredbody (`self.KinectPoseableMesh`))))

(fn `UserConstructionScript`)