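; BP_IR_Opacity shows the live Kinect infrared camera frame on a plane through an opacity material.
; On BeginPlay it creates a dynamic instance of M_Kinect_Opacity_Inst, binds the IR frame as its texture and enables updates for that camera.
; The Up and Down keys step the Depth variable, which drives the material's Scale parameter.
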(event `self.ReceiveBeginPlay`
  (bind _returnvalue (`KinectInterfaceComponent.GetCameraFrame` (`self.KinectInterface`) "IR"))
  (bind _returnvalue_2 (`PrimitiveComponent.CreateDynamicMaterialInstance` (`self.Plane`) 0 "/Game/Materials/Introduction/M_Kinect_Opacity_Inst.M_Kinect_Opacity_Inst" "Texture"))
  (set `self.DepthMat` _returnvalue_2)
  (`MaterialInstanceDynamic.SetTextureParameterValue` _returnvalue_2 "Texture" _returnvalue)
  (`KinectInterfaceComponent.SetCameraFrameIsUpdating` (`self.KinectInterface`) "IR" true))

(event `Key|Up`
  (params (Key :type "Key Structure"))
  (:`Pressed`
    (bind _output_get (set `self.depth` (+ (`self.depth`) 10.0)))
    (`MaterialInstanceDynamic.SetScalarParameterValue` (`self.DepthMat`) "Scale" _output_get)))

(event `Key|Down`
  (params (Key :type "Key Structure"))
  (:`Pressed`
    (bind _output_get (set `self.depth` (- (`self.depth`) 10.0)))
    (`MaterialInstanceDynamic.SetScalarParameterValue` (`self.DepthMat`) "Scale" _output_get)))

(fn `UserConstructionScript`)