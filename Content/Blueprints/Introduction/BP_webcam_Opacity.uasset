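; Introduction actor that shows a live webcam feed on a plane, with brightness adjustable from the keyboard.
; BeginPlay puts a dynamic instance of the media material on the plane, lists video and webcam capture devices, and opens the first in FrontMediaPlayer.
; Once opened, the player selects a video track and plays, retrying once after a short delay on failure.
; Up and Down keys step the Depth value that drives the material's Brightness parameter.
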(event `Key|Up`
  (params (Key :type "Key Structure"))
  (:`Pressed`
    (bind _output_get (set `self.depth` (+ (`self.depth`) 0.1)))
    (`MaterialInstanceDynamic.SetScalarParameterValue` (`self.DepthMat`) "Brightness" _output_get)))

(event `Key|Down`
  (params (Key :type "Key Structure"))
  (:`Pressed`
    (bind _output_get (set `self.depth` (- (`self.depth`) 0.1)))
    (`MaterialInstanceDynamic.SetScalarParameterValue` (`self.DepthMat`) "Brightness" _output_get)))

(event `self.ReceiveBeginPlay`
  (bind _capturedevices (`self.CaptureDevices`))
  (bind _returnvalue (`PrimitiveComponent.CreateDynamicMaterialInstance` (`self.Plane`) 0 "/Game/Blueprints/Introduction/NewMediaPlayer_Video_Mat_Inst.NewMediaPlayer_Video_Mat_Inst" "Texture"))
  (bind _output_get (set `self.DepthMat` _returnvalue))
  (`PrimitiveComponent.SetMaterial` (`self.Plane`) 0 _output_get)
  (bind _outdevices (`MediaBlueprintFunctionLibrary.EnumerateVideoCaptureDevices` -1))
  (set `self.CaptureDevices` _outdevices)
  (bind _outdevices_2 (`MediaBlueprintFunctionLibrary.EnumerateWebcamCaptureDevices` -1))
  (for _array_element _outdevices_2
    (`KismetArrayLibrary.Array_Add` _capturedevices _array_element))
  (for (_array_element_2 _array_index) _capturedevices
    (bind (_displayname _url) (break `MediaCaptureDevice` _array_element_2))
    (`KismetSystemLibrary.PrintString` (`KismetTextLibrary.Conv_TextToString` _displayname))
    (switch `int` _array_index
      (:`0`
        (`MediaPlayer.OpenUrl` (`self.FrontMediaPlayer`) _url)
        (add `MediaPlayer.OnMediaOpened` (`self.FrontMediaPlayer`) (delegate `OnMediaOpened_1`))))))

(event `OnMediaOpened_1`
  (params (OpenedUrl :type String))
  (bind _frontmediaplayer (`self.FrontMediaPlayer`))
  (`MediaPlayer.SelectTrack` _frontmediaplayer "Video" 1)
  (bind _returnvalue (`MediaPlayer.Play` _frontmediaplayer))
  (if (not _returnvalue)
    (`KismetSystemLibrary.Delay` 0.5)
    (`MediaPlayer.Play` _frontmediaplayer)))

(fn `UserConstructionScript`)